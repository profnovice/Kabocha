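; BP_SaveGame is a save game Blueprint that coordinates saving and loading object data per level.
; SaveAllData messages each saveable object to save its data, passing itself and a level reference, then marks that level's LevelStates entry valid.
; LoadDataForRequester sends the matching load message to a single requester.
; Serialization is delegated to the objects through these messages, so this asset holds no object-specific logic.
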(fn SaveAllData
  (params (SaveableObjects :type Array%20of%20Object%20Object%20References) (LevelDataRef :type Integer))
  (for _array_element SaveableObjects
    (Class|BPISaveable|SaveObjectData(Message) _array_element self LevelDataRef))
  (Utilities|Struct|SetmembersinST_LevelData (Utilities|Array|Get(acopy) (Variables|Default|GetLevelStates) LevelDataRef) true)
  (return))

(fn LoadDataforRequester
  (params (Requester :type Object%20Object%20Reference) (LevelDataRef :type Integer))
  (Class|BPISaveable|LoadObjectData(Message) Requester self LevelDataRef)
  (return))