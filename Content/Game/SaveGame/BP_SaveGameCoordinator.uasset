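; BP_SaveGameCoordinator is an actor that saves and restores the BP_Item actors in a level.
; On BeginPlay it passes itself to the GameInstance with a load request.
; SaveObjectData rebuilds that level's entry in the save game's LevelStates from every BP_Item present.
; LoadObjectData, if that entry is valid, destroys all existing items and respawns them from the saved item structs and transforms.
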(event EventBeginPlay
  (Class|BPIPersistance|RequestLoad(Message) (Game|GetGameInstance) self))

(event Collision|EventActorBeginOverlap
  (params (OtherActor :type Actor%20Object%20Reference)))

(event EventTick
  (params (DeltaSeconds :type Float%20%28single-precision%29)))

(event EventLoadObjectData
  (params (SaveGameRef :type BP%20Save%20Game%20Object%20Reference) (LevelDataRef :type Integer))
  (bind _levelstates (Variables|/Game/Game/SaveGame/BP_SaveGame.BP_SaveGame_C|GetLevelStates SaveGameRef))
  (bind _output (Utilities|Array|Get(acopy) _levelstates LevelDataRef))
  (if (.isvalid _output)
    (bind _outactors (Actor|GetAllActorsOfClass "/Game/Game/Blueprints/Actors/BP_Item.BP_Item_C"))
    (for _array_element _outactors
      (Actor|DestroyActor _array_element))
    (for _array_element_2 (.itemsinleveldata _output)
      (Game|SpawnActorfromClass "/Game/Game/Blueprints/Actors/BP_Item.BP_Item_C" (.itemtransform _array_element_2) "AlwaysSpawn" "MultiplyWithRoot" 0 (.item _array_element_2) 0))))

(event EventSaveObjectData
  (params (SaveGameRef :type BP%20Save%20Game%20Object%20Reference) (LevelDataRef :type Integer))
  (bind _levelstates (Variables|/Game/Game/SaveGame/BP_SaveGame.BP_SaveGame_C|GetLevelStates SaveGameRef))
  (bind _output (Utilities|Array|Get(acopy) _levelstates LevelDataRef))
  (bind _outactors (Actor|GetAllActorsOfClass "/Game/Game/Blueprints/Actors/BP_Item.BP_Item_C"))
  (Utilities|Array|Clear (.itemsinleveldata _output))
  (for _array_element _outactors
    (bind _itemdata (Default|GetSTItemsinLevelData _array_element))
    (Utilities|Array|Add (.itemsinleveldata _output) _itemdata)))

(fn ConstructionScript)