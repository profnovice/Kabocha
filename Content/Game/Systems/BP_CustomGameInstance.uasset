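; Game instance that owns the BP_SaveGame object and handles creating, loading and saving it in a single slot.
; Loading and saving run sync or async and notify on success; a missing save yields a fresh object.
; Save requests pass all BPI_Saveable actors to the save object with the current level's LevelStates index, found or added by name, then write the slot.
; Load requests restore one requester from that level's entry.
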(event Custom|SaveGameEvent
  (params (Async :type Boolean))
  (if Async
    (|AsyncSaveGametoSlot (Variables|Default|GetSaveGame) (Variables|Default|GetSaveGameSlotName)
      (:Completed
        (Default|CallGameIsSaved (Variables|Default|GetSaveGame))))
    (else
      (SaveGame|SaveGametoSlot (Variables|Default|GetSaveGame) (Variables|Default|GetSaveGameSlotName))
      (Default|CallGameIsSaved (Variables|Default|GetSaveGame)))))

(event Custom|CreateSaveGame
  (bind _savegameslotname (Variables|Default|GetSaveGameSlotName))
  (bind _returnvalue (SaveGame|DoesSaveGameExist _savegameslotname))
  (if _returnvalue
    (SaveGame|DeleteGameinSlot _savegameslotname))
  (bind _returnvalue_2 (SaveGame|CreateSaveGameObject "/Game/Game/SaveGame/BP_SaveGame.BP_SaveGame_C"))
  (Variables|Default|SetSaveGame _returnvalue_2))

(event Custom|LoadGame
  (params (Async :type Boolean))
  (bind _returnvalue (SaveGame|DoesSaveGameExist (Variables|Default|GetSaveGameSlotName)))
  (if _returnvalue
    (if Async
      (bind _savegame (|AsyncLoadGamefromSlot (Variables|Default|GetSaveGameSlotName))
        (:Completed
          (bind _asbp_save_game (Utilities|Casting|CastToBP_SaveGame _savegame))
          (Variables|Default|SetSaveGame _asbp_save_game)
          (Default|CallGameLoaded (Variables|Default|GetSaveGame))))
      (else
        (bind _returnvalue_2 (SaveGame|LoadGamefromSlot (Variables|Default|GetSaveGameSlotName)))
        (bind _asbp_save_game_2 (Utilities|Casting|CastToBP_SaveGame _returnvalue_2))
        (Variables|Default|SetSaveGame _asbp_save_game_2)
        (Default|CallGameLoaded (Variables|Default|GetSaveGame))))
    (else
      (bind _returnvalue_3 (SaveGame|CreateSaveGameObject "/Game/Game/SaveGame/BP_SaveGame.BP_SaveGame_C"))
      (Variables|Default|SetSaveGame _returnvalue_3))))

(event EventRequestSave
  (params (Async :type Boolean))
  (bind _savegame (Variables|Default|GetSaveGame))
  (bind _returnvalue (Game|GetCurrentLevelName true))
  (bind _output_get (Variables|/Game/Game/SaveGame/BP_SaveGame.BP_SaveGame_C|SetSaveLevelName _savegame _returnvalue))
  (bind _matchingleveldata (CallFunction|GetorAddLevelIndex _output_get (Variables|/Game/Game/SaveGame/BP_SaveGame.BP_SaveGame_C|GetLevelStates _savegame)))
  (bind _outactors (Actor|GetAllActorswithInterface "/Game/Game/Blueprints/Interfaces/BPI_Saveable.BPI_Saveable_C"))
  (Default|SaveAllData (Variables|Default|GetSaveGame) _outactors _matchingleveldata)
  (CallFunction|SaveGameEvent Async))

(event EventRequestLoad
  (params (Requester :type Object%20Object%20Reference))
  (bind _returnvalue (Game|GetCurrentLevelName true))
  (bind _matchingleveldata (CallFunction|GetorAddLevelIndex _returnvalue (Variables|/Game/Game/SaveGame/BP_SaveGame.BP_SaveGame_C|GetLevelStates (Variables|Default|GetSaveGame))))
  (Default|LoadDataforRequester (Variables|Default|GetSaveGame) Requester _matchingleveldata))

(fn GetorAddLevelData
  (params (LevelName :type String) (LevelDataArray :type Array%20of%20ST%20Level%20Data%20Structures) (IsSaving :type Boolean))
  (bind _st_leveldata (Utilities|Struct|MakeST_LevelData LevelName IsSaving "()"))
  (for _array_element LevelDataArray
    (if (Utilities|Enum|Equal(Enum) (.LevelName (Utilities|Struct|BreakST_LevelData _array_element)) LevelName)
      (return _array_element)))
  (Utilities|Array|Add LevelDataArray _st_leveldata)
  (return _st_leveldata))

(fn GetorAddLevelIndex
  (params (LevelName :type String) (LevelDataArray :type Array%20of%20ST%20Level%20Data%20Structures))
  (for (_array_element _array_index) LevelDataArray
    (if (Utilities|Enum|Equal(Enum) (.LevelName (Utilities|Struct|BreakST_LevelData _array_element)) LevelName)
      (return _array_index)))
  (bind _returnvalue (Utilities|Array|Add LevelDataArray (Utilities|Struct|MakeST_LevelData LevelName false "()")))
  (return _returnvalue))