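; Base enemy character Blueprint that roams the level and reacts to damage and death.
; On BeginPlay it loops through PatrolPoints via AIMoveTo, lingering at each, or wanders to random reachable points if none are set.
; HealthComponent events drive pitch-randomized hurt grunts and a one-time death.
; Death optionally spawns a BP_Item drop from DT_Items, then ragdolls the mesh with an upward impulse, stops patrolling and destroys the actor after a delay.
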(event OnDamageTaken(HealthComponent)
  (if (not (Variables|/Game/Game/Blueprints/Components/HealthComponent.HealthComponent_C|GetIsDead (Variables|Default|GetHealthComponent)))
    (Audio|PlaySoundatLocation "/Game/Game/Audio/SFX/weird-grunt-85631.weird-grunt-85631" (Transformation|GetActorLocation) "0, 0, 0" 1.0 (Math|Random|RandomFloatinRange 0.5 1.5) 0.0 0 0 0 0)))

(event OnDeath(HealthComponent)
  (bind _mesh (Variables|Character|GetMesh))
  (bind _row_name (Variables|Default|GetRow%20Name))
  (Utilities|FlowControl|DoOnce false
    (:Completed
      (if (and (!= _row_name "Null") (Variables|Default|GetShould%20Drop))
        (bind _returnvalue (Utilities|GetDataTableRow "/Game/Game/Systems/Inventory/DT_Items.DT_Items" _row_name)
          (:then
            (Game|SpawnActorfromClass "/Game/Game/Blueprints/Actors/BP_Item.BP_Item_C" (Transformation|GetWorldTransform (Variables|Collision|GetCapsuleComponent)) "AlwaysSpawn" "MultiplyWithRoot" self _returnvalue 0))))
      (Audio|Components|Audio|Stop (Variables|Character|GetMesh))
      (Components|SkeletalMesh|SetAnimInstanceClass (Variables|Character|GetMesh) 0)
      (Collision|SetCollisionEnabled _mesh "QueryAndPhysics")
      (Physics|SetSimulatePhysics _mesh true)
      (Physics|AddImpulse _mesh "0.000000,0.000000,2000.000000" "None" true)
      (Collision|SetCollisionEnabled (Variables|Collision|GetCapsuleComponent) "NoCollision")
      (Variables|Default|SetShouldPatrol false)
      (Components|Movement|StopMovementImmediately (Variables|Character|GetCharacterMovement))
      (Utilities|FlowControl|Delay 1e+01)
      (Actor|DestroyActor))))

(event Custom|Wander
  (if (Variables|Default|GetShouldPatrol)
    (AI|AIMoveTo self (.RandomLocation (AI|Navigation|GetRandomReachablePointinRadius (Transformation|GetActorLocation) 1e+03 0 0)) 0 5.0 false
      (:OnSuccess
        _)
      (:OnFail
        _))
    (Utilities|FlowControl|Delay 2.0)
    (CallFunction|Wander)))

(event Custom|Patrol
  (if (Variables|Default|GetShouldPatrol)
    (AI|AIMoveTo self "0, 0, 0" (Utilities|Array|Get(acopy) (Variables|Default|GetPatrolPoints) (Variables|Default|GetIncrement)) 5.0 false
      (:OnSuccess
        _)
      (:OnFail
        _))
    (Utilities|IsValid (Variables|/Game/Game/Blueprints/Actors/BP_PatrolPoint.BP_PatrolPoint_C|GetCustomAnim (Utilities|Array|Get(acopy) (Variables|Default|GetPatrolPoints) (Variables|Default|GetIncrement)))
      (:Is%20Valid
        _)
      (:Is%20Not%20Valid
        _))
    (Utilities|FlowControl|Delay (Variables|/Game/Game/Blueprints/Actors/BP_PatrolPoint.BP_PatrolPoint_C|GetTimeToLinger (Utilities|Array|Get(acopy) (Variables|Default|GetPatrolPoints) (Variables|Default|GetIncrement))))
    (bind _result (Math|Integer|IncrementInt (Variables|Default|GetIncrement))
      (:%20%20
        (bind _output_get (Variables|Default|SetIncrement _result))
        (if (>= _output_get (Utilities|Array|Length (Variables|Default|GetPatrolPoints)))
          (Variables|Default|SetIncrement 0))
        (CallFunction|Patrol)))))

(event EventBeginPlay
  (if (Utilities|Array|IsNotEmpty (Variables|Default|GetPatrolPoints))
    (CallFunction|Patrol)
    (else
      (CallFunction|Wander))))

(fn ConstructionScript)