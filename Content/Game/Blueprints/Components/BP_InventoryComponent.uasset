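; Inventory component that stores a size-limited item array, shows it in a WB_Inventory widget and toggles that widget by input.
; Adding merges same-named stackables within their carry limit, while charging deducts a quantity from one matching stack.
; Dropping spawns a BP_Item ahead of the owner with a sound, one unit for physical items, otherwise the whole stack.
; A selected index wraps while cycling, and item changes reload the widget.
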(event Custom|RemoveItem
  (bind _returnvalue (Components|GetOwner))
  (bind _items (Variables|Default|GetItems))
  (bind _returnvalue_2 (Transformation|GetActorForwardVector _returnvalue))
  (bind _returnvalue_3 (Transformation|GetActorTransform _returnvalue))
  (bind (_location _rotation _scale) (Math|Transform|BreakTransform _returnvalue_3))
  (bind _returnvalue_4 (* _returnvalue_2 "100.000000,100.000000,100.000000"))
  (bind _returnvalue_5 (+ _location _returnvalue_4))
  (bind _returnvalue_6 (Math|Transform|MakeTransform _returnvalue_5 _rotation _scale))
  (if (> (Utilities|Array|Length _items) 0)
    (if (.IsPhysical (Utilities|Struct|BreakST_Item (Utilities|Array|Get(acopy) _items (Variables|Default|GetInventoryIndexOfInterest))))
      (Game|SpawnActorfromClass "/Game/Game/Blueprints/Actors/BP_Item.BP_Item_C" _returnvalue_6 "AlwaysSpawn" "MultiplyWithRoot" 0 (Utilities|Struct|MakeST_Item (.Name (Utilities|Struct|BreakST_Item (Utilities|Array|Get(acopy) _items (Variables|Default|GetInventoryIndexOfInterest)))) (.Stackable (Utilities|Struct|BreakST_Item (Utilities|Array|Get(acopy) _items (Variables|Default|GetInventoryIndexOfInterest)))) 1 (.Thumbnail (Utilities|Struct|BreakST_Item (Utilities|Array|Get(acopy) _items (Variables|Default|GetInventoryIndexOfInterest)))) (.Mesh (Utilities|Struct|BreakST_Item (Utilities|Array|Get(acopy) _items (Variables|Default|GetInventoryIndexOfInterest)))) (.PickupSound (Utilities|Struct|BreakST_Item (Utilities|Array|Get(acopy) _items (Variables|Default|GetInventoryIndexOfInterest)))) (.MaxCarryQuantity (Utilities|Struct|BreakST_Item (Utilities|Array|Get(acopy) _items (Variables|Default|GetInventoryIndexOfInterest)))) (.IsPhysical (Utilities|Struct|BreakST_Item (Utilities|Array|Get(acopy) _items (Variables|Default|GetInventoryIndexOfInterest)))) (.DropSound (Utilities|Struct|BreakST_Item (Utilities|Array|Get(acopy) _items (Variables|Default|GetInventoryIndexOfInterest))))) 0)
      (Audio|PlaySoundatLocation (.DropSound (Utilities|Struct|BreakST_Item (Utilities|Array|Get(acopy) _items (Variables|Default|GetInventoryIndexOfInterest)))) _location "0, 0, 0" 1.0 1.0 0.0 0 0 0 0)
      (if (> (.Quantity (Utilities|Struct|BreakST_Item (Utilities|Array|Get(acopy) _items (Variables|Default|GetInventoryIndexOfInterest)))) 1)
        (Utilities|Array|SetArrayElem (Variables|Default|GetItems) (Variables|Default|GetInventoryIndexOfInterest) (Utilities|Struct|MakeST_Item (.Name (Utilities|Struct|BreakST_Item (Utilities|Array|Get(acopy) _items (Variables|Default|GetInventoryIndexOfInterest)))) (.Stackable (Utilities|Struct|BreakST_Item (Utilities|Array|Get(acopy) _items (Variables|Default|GetInventoryIndexOfInterest)))) (- (.Quantity (Utilities|Struct|BreakST_Item (Utilities|Array|Get(acopy) _items (Variables|Default|GetInventoryIndexOfInterest)))) 1) (.Thumbnail (Utilities|Struct|BreakST_Item (Utilities|Array|Get(acopy) _items (Variables|Default|GetInventoryIndexOfInterest)))) (.Mesh (Utilities|Struct|BreakST_Item (Utilities|Array|Get(acopy) _items (Variables|Default|GetInventoryIndexOfInterest)))) (.PickupSound (Utilities|Struct|BreakST_Item (Utilities|Array|Get(acopy) _items (Variables|Default|GetInventoryIndexOfInterest)))) (.MaxCarryQuantity (Utilities|Struct|BreakST_Item (Utilities|Array|Get(acopy) _items (Variables|Default|GetInventoryIndexOfInterest)))) (.IsPhysical (Utilities|Struct|BreakST_Item (Utilities|Array|Get(acopy) _items (Variables|Default|GetInventoryIndexOfInterest)))) (.DropSound (Utilities|Struct|BreakST_Item (Utilities|Array|Get(acopy) _items (Variables|Default|GetInventoryIndexOfInterest))))))
        (else
          (Utilities|Array|RemoveIndex _items (Variables|Default|GetInventoryIndexOfInterest) :!label _label)
          (Variables|Default|SetInventoryIndexOfInterest (Math|Integer|Clamp(Integer) (Math|Integer|Clamp(Integer) (Variables|Default|GetInventoryIndexOfInterest) 0 (- (Utilities|Array|Length (Variables|Default|GetItems)) 1)) 0 (Variables|Default|GetMaxInventorySize)))))
      (else
        (Game|SpawnActorfromClass "/Game/Game/Blueprints/Actors/BP_Item.BP_Item_C" _returnvalue_6 "AlwaysSpawn" "MultiplyWithRoot" 0 (Utilities|Struct|MakeST_Item (.Name (Utilities|Struct|BreakST_Item (Utilities|Array|Get(acopy) _items (Variables|Default|GetInventoryIndexOfInterest)))) (.Stackable (Utilities|Struct|BreakST_Item (Utilities|Array|Get(acopy) _items (Variables|Default|GetInventoryIndexOfInterest)))) (.Quantity (Utilities|Struct|BreakST_Item (Utilities|Array|Get(acopy) _items (Variables|Default|GetInventoryIndexOfInterest)))) (.Thumbnail (Utilities|Struct|BreakST_Item (Utilities|Array|Get(acopy) _items (Variables|Default|GetInventoryIndexOfInterest)))) (.Mesh (Utilities|Struct|BreakST_Item (Utilities|Array|Get(acopy) _items (Variables|Default|GetInventoryIndexOfInterest)))) (.PickupSound (Utilities|Struct|BreakST_Item (Utilities|Array|Get(acopy) _items (Variables|Default|GetInventoryIndexOfInterest)))) (.MaxCarryQuantity (Utilities|Struct|BreakST_Item (Utilities|Array|Get(acopy) _items (Variables|Default|GetInventoryIndexOfInterest)))) (.IsPhysical (Utilities|Struct|BreakST_Item (Utilities|Array|Get(acopy) _items (Variables|Default|GetInventoryIndexOfInterest)))) (.DropSound (Utilities|Struct|BreakST_Item (Utilities|Array|Get(acopy) _items (Variables|Default|GetInventoryIndexOfInterest))))) 0)
        (Audio|PlaySoundatLocation (.DropSound (Utilities|Struct|BreakST_Item (Utilities|Array|Get(acopy) _items (Variables|Default|GetInventoryIndexOfInterest)))) _location "0, 0, 0" 1.0 1.0 0.0 0 0 0 0)
        (goto _label)))
    (Default|LoadInventory (Variables|Default|GetInventoryWidget) self (Variables|Default|GetInventoryIndexOfInterest))))

(event Custom|RefreshInventory
  (Default|LoadInventory (Variables|Default|GetInventoryWidget) self (Variables|Default|GetInventoryIndexOfInterest)))

(event Input|EnhancedActionEvents|EnhancedInputActionIA_Inventory
  (params (ActionValue :type Boolean) (ElapsedSeconds :type Float%20%28double-precision%29) (TriggeredSeconds :type Float%20%28double-precision%29) (InputAction :type Input%20Action%20Object%20Reference :default "/Game/Game/Systems/Input/Actions/IA_Inventory.IA_Inventory"))
  (bind _inventorywidget (Variables|Default|GetInventoryWidget))
  (:Started
    (if (Widget|IsVisible _inventorywidget)
      (Widget|RemovefromParent _inventorywidget)
      (else
        (UserInterface|Viewport|AddtoViewport _inventorywidget 0)
        (CallFunction|RefreshInventory)))))

(event Input|EnhancedActionEvents|EnhancedInputActionIA_DropItem
  (params (ActionValue :type Boolean) (ElapsedSeconds :type Float%20%28double-precision%29) (TriggeredSeconds :type Float%20%28double-precision%29) (InputAction :type Input%20Action%20Object%20Reference :default "/Game/Game/Systems/Input/Actions/IA_DropItem.IA_DropItem"))
  (:Started
    (CallFunction|RemoveItem)))

(event EventBeginPlay
  (Utilities|FlowControl|Sequence
    (:then_0
      (bind _returnvalue (UserInterface|CreateWidget "/Game/Game/UI/WB_Inventory.WB_Inventory_C"))
      (Variables|Default|SetInventoryWidget _returnvalue))
    (:then_1
      (Utilities|Array|Resize (Variables|Default|GetItems) 0)
      (Default|LoadInventory (Variables|Default|GetInventoryWidget) self (Variables|Default|GetInventoryIndexOfInterest)))
    (:then_2
      (if (Widget|IsVisible (Variables|Default|GetInventoryWidget))
        (Widget|RemovefromParent (Variables|Default|GetInventoryWidget))
        (else
          (UserInterface|Viewport|AddtoViewport (Variables|Default|GetInventoryWidget) 0)
          (CallFunction|RefreshInventory))))))

(event EventTick
  (params (DeltaSeconds :type Float%20%28single-precision%29)))

(fn AddItemtoInventory
  (params (Item :type ST%20Item%20Structure))
  (bind _items (Variables|Default|GetItems))
  (LocalVariables|SetNewItem Item)
  (for (_array_element _array_index) (Variables|Default|GetItems)
    (if (not (LocalVariables|GetIsConsumed))
      (if (Utilities|Enum|Equal(Enum) (.Name (Utilities|Struct|BreakST_Item _array_element)) (.Name (Utilities|Struct|BreakST_Item (LocalVariables|GetNewItem))))
        (if (and (.Stackable (Utilities|Struct|BreakST_Item (LocalVariables|GetNewItem))) (<= (+ (.Quantity (Utilities|Struct|BreakST_Item _array_element)) (.Quantity (Utilities|Struct|BreakST_Item (LocalVariables|GetNewItem)))) (.MaxCarryQuantity (Utilities|Struct|BreakST_Item (LocalVariables|GetNewItem)))))
          (Utilities|Array|SetArrayElem (Variables|Default|GetItems) _array_index (Utilities|Struct|MakeST_Item (.name (LocalVariables|GetNewItem)) (.stackable (LocalVariables|GetNewItem)) (+ (.Quantity (Utilities|Struct|BreakST_Item _array_element)) (.Quantity (Utilities|Struct|BreakST_Item (LocalVariables|GetNewItem)))) (.thumbnail (LocalVariables|GetNewItem)) (.mesh (LocalVariables|GetNewItem)) (.pickupsound (LocalVariables|GetNewItem)) (.maxcarryquantity (LocalVariables|GetNewItem)) (.isphysical (LocalVariables|GetNewItem)) (.dropsound (LocalVariables|GetNewItem))))
          (Default|LoadInventory (Variables|Default|GetInventoryWidget) self)
          (LocalVariables|SetIsConsumed true)))))
  (if (LocalVariables|GetIsConsumed)
    (return true)
    (elif (< (Utilities|Array|Length _items) (Variables|Default|GetMaxInventorySize))
      (Utilities|Array|Add _items (LocalVariables|GetNewItem))
      (LocalVariables|SetIsConsumed true)
      (Default|LoadInventory (Variables|Default|GetInventoryWidget) self)
      (return true)
      (else
        (return false)))))

(fn SetInventoryIndexOfInterest
  (params (Change :type Integer))
  (bind _items (Variables|Default|GetItems))
  (bind _returnvalue (Utilities|Array|Length _items))
  (if (>= (+ Change (Variables|Default|GetInventoryIndexOfInterest)) (Utilities|Array|Length (Variables|Default|GetItems)))
    (Variables|Default|SetInventoryIndexOfInterest 0)
    (elif (< (+ Change (Variables|Default|GetInventoryIndexOfInterest)) 0)
      (Variables|Default|SetInventoryIndexOfInterest (Math|Integer|Clamp(Integer) (Math|Integer|Clamp(Integer) _returnvalue 0 (- _returnvalue 1)) 0 (Variables|Default|GetMaxInventorySize)))
      (else
        (Variables|Default|SetInventoryIndexOfInterest (Math|Integer|Clamp(Integer) (Math|Integer|Clamp(Integer) (+ Change (Variables|Default|GetInventoryIndexOfInterest)) 0 (- _returnvalue 1)) 0 (Variables|Default|GetMaxInventorySize))))))
  (Default|LoadInventory (Variables|Default|GetInventoryWidget) self (Variables|Default|GetInventoryIndexOfInterest))
  (Development|PrintText (Utilities|Text|ToText(Integer) (Variables|Default|GetInventoryIndexOfInterest))))

(fn AttempttoChargeAmount
  (params (Quanity :type Integer) (Item :type ST%20Item%20Structure))
  (bind _items (Variables|Default|GetItems))
  (LocalVariables|SetLocalQuanity Quanity)
  (for (_array_element _array_index) (Variables|Default|GetItems)
    (if (not (LocalVariables|GetSuccessful))
      (if (Utilities|Enum|Equal(Enum) (.Name (Utilities|Struct|BreakST_Item _array_element)) (.Name (Utilities|Struct|BreakST_Item Item)))
        (if (<= (LocalVariables|GetLocalQuanity) (.Quantity (Utilities|Struct|BreakST_Item _array_element)))
          (if (> (- (.Quantity (Utilities|Struct|BreakST_Item _array_element)) (LocalVariables|GetLocalQuanity)) 0)
            (Utilities|Array|SetArrayElem _items _array_index (Utilities|Struct|MakeST_Item (.Name (Utilities|Struct|BreakST_Item _array_element)) (.Stackable (Utilities|Struct|BreakST_Item _array_element)) (- (.Quantity (Utilities|Struct|BreakST_Item _array_element)) (LocalVariables|GetLocalQuanity)) (.Thumbnail (Utilities|Struct|BreakST_Item _array_element)) (.Mesh (Utilities|Struct|BreakST_Item _array_element)) (.PickupSound (Utilities|Struct|BreakST_Item _array_element)) (.MaxCarryQuantity (Utilities|Struct|BreakST_Item _array_element)) (.IsPhysical (Utilities|Struct|BreakST_Item _array_element)) (.DropSound (Utilities|Struct|BreakST_Item _array_element))))
            (LocalVariables|SetSuccessful true)
            (else
              (Utilities|Array|RemoveIndex _items _array_index)
              (LocalVariables|SetSuccessful true)))))))
  (Variables|Default|SetInventoryIndexOfInterest (Math|Integer|Clamp(Integer) (Math|Integer|Clamp(Integer) (Variables|Default|GetInventoryIndexOfInterest) 0 (- (Utilities|Array|Length (Variables|Default|GetItems)) 1)) 0 (Variables|Default|GetMaxInventorySize)))
  (Default|LoadInventory (Variables|Default|GetInventoryWidget) self (Variables|Default|GetInventoryIndexOfInterest))
  (return (LocalVariables|GetSuccessful)))