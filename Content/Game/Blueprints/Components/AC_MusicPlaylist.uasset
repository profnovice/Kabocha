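; Music playlist component that plays songs from a data table as 2D audio in shuffled order.
; On BeginPlay it collects unique songs, shuffles them, then spawns a persistent audio component with a starter sound whose finish event chains into PlayNextSong.
; When the index wraps, the list reshuffles, swapping the first entry if it matches the previous cycle's last to avoid back-to-back repeats.
; A debug key (M) skips to the next song.
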(event Custom|ReshufflePlaylist
  (bind _playlist (Variables|Default|GetPlaylist))
  (bind _returnvalue (Utilities|Array|LastIndex _playlist))
  (Utilities|Array|Shuffle _playlist)
  (if (== (Variables|Default|GetPrevLastSong) (Utilities|Array|Get(acopy) _playlist))
    (Utilities|Array|Swap _playlist 0 (Math|Random|RandomIntegerinRange 1 _returnvalue)))
  (Variables|Default|SetPrevLastSong (Utilities|Array|Get(acopy) _playlist _returnvalue)))

(event Custom|PlayNextSong
  (bind _audio (Variables|Default|GetAudio))
  (Audio|Components|Audio|SetSound _audio (Utilities|Array|Get(acopy) (Variables|Default|GetPlaylist) (Variables|Default|GetCurrentSongIndex)))
  (Audio|Components|Audio|Play _audio 0.0)
  (if (> (+ (Variables|Default|GetCurrentSongIndex) 1) (Utilities|Array|LastIndex (Variables|Default|GetPlaylist)))
    (Variables|Default|SetCurrentSongIndex 0)
    (CallFunction|ReshufflePlaylist)
    (else
      (Variables|Default|SetCurrentSongIndex (+ (Variables|Default|GetCurrentSongIndex) 1)))))

(event EventBeginPlay
  (Utilities|FlowControl|Sequence
    (:then_0
      (bind _outrownames (DataTable|GetDataTableRowNames "/Game/Game/Audio/Playlist.Playlist"))
      (for _array_element _outrownames
        (bind _returnvalue (Utilities|GetDataTableRow "/Game/Game/Audio/Playlist.Playlist" _array_element)
          (:then
            (Utilities|Array|AddUnique (Variables|Default|GetPlaylist) (Utilities|Struct|BreakST_Song _returnvalue))))))
    (:then_1
      (CallFunction|ReshufflePlaylist))
    (:then_2
      (bind _returnvalue_2 (Audio|SpawnSound2D "/Game/Game/Audio/SFX/analog-appliance-button-15-186961.analog-appliance-button-15-186961" 1.0 1.0 0.0 0 false false))
      (Variables|Default|SetAudio _returnvalue_2)
      (EventDispatchers|BindEventtoOnAudioFinished (Variables|Default|GetAudio) (delegate Custom|PlayNextSong)))))

(event EventTick
  (params (DeltaSeconds :type Float%20%28single-precision%29)))

(event Input|KeyboardEvents|DebugKeyM
  (params (Key :type Key%20Structure :default "None") (ActionValue :type Input%20Action%20Value%20Structure))
  (:Pressed
    (Development|PrintString (Utilities|String|ToString(Integer) (Variables|Default|GetCurrentSongIndex)))
    (CallFunction|PlayNextSong)))