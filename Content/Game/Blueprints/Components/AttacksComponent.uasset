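; AttacksComponent is a component that gives its owner a forward attack, damaging an actor that has a HealthComponent.
; ForwardAttackFunc sphere-traces a short distance along the passed camera's forward vector, ignoring the owner and gathering unique HealthComponents from the hits.
; Only the first gathered component receives TakeDamageMessage, with no empty-array check, before the list is cleared.
; The ForwardAttack and AOEAttack events are empty, and a single-trace variant sits unconnected.
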(event Custom|ForwardAttack)

(event Custom|AOEAttack)

(fn ForwardAttackFunc
  (params (Cam :type Arrow%20Component%20Object%20Reference))
  (bind _returnvalue (Transformation|GetWorldTransform Cam))
  (bind _outhits (Collision|MultiSphereTraceForObjects (.location _returnvalue) (+ (.location _returnvalue) (* (Math|Vector|GetForwardVector (.rotation _returnvalue)) "500.000000,500.000000,500.000000")) 0.0 (Variables|Default|GetObject%20Types) false (Utilities|Array|MakeArray (Components|GetOwner)) "None"))
  (for _array_element _outhits
    (Utilities|IsValid (Actor|GetComponentbyClass (.hitactor _array_element) "/Game/Game/Blueprints/Components/HealthComponent.HealthComponent_C")
      (:Is%20Valid
        (Utilities|Array|AddUnique (Variables|Default|GetHealthCompHit) (Actor|GetComponentbyClass (.hitactor _array_element) "/Game/Game/Blueprints/Components/HealthComponent.HealthComponent_C")))))
  (Class|BPIHealthComponent|TakeDamage(Message) (Utilities|Array|Get(acopy) (Variables|Default|GetHealthCompHit)) 25.0)
  (Utilities|Array|Clear (Variables|Default|GetHealthCompHit)))