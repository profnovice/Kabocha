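; Interactable actor that toggles the time of day by switching the level's Directional Light between two fixed rotations.
; BeginPlay finds the light, sets its starting rotation and plays the Orbit timeline, which yaws the Terra component.
; Each Interact alternates through a FlipFlop, playing a sound, snapping the light and running a timeline that counter-rotates Cube2 and Cube8, reversing their directions each time.
; An unconnected Timeline_0 branch never runs.
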(event EventBeginPlay
  (bind _returnvalue (Actor|GetActorOfClass "/Script/Engine.DirectionalLight"))
  (Variables|Default|SetLight _returnvalue)
  (Transformation|SetActorRotation (Variables|Default|GetLight) "-90.000000,0.000000,0.000000")
  (bind _newtrack_1 (Timeline|Orbit Play)
    (:Update
      (Transformation|SetRelativeRotation (Variables|Default|GetTerra) (Math|Rotator|MakeRotator 0.0 0.0 _newtrack_1) false false))))

(event EventInteract
  (params (Interactor :type Actor%20Object%20Reference))
  (bind _light (Variables|Default|GetLight))
  (Utilities|FlowControl|FlipFlop
    (:A
      (Audio|PlaySoundatLocation "/Game/Game/Audio/SFX/drop-sound-effect-240899.drop-sound-effect-240899" (Transformation|GetActorLocation) "0, 0, 0" 1.0 1.0 0.0 0 0 0 0)
      (Transformation|SetActorRotation _light)
      (bind _doublespin (Timeline|ActivateTimeline PlayFromStart)
        (:Update
          (Transformation|SetRelativeRotation (Variables|Default|GetCube2) (Math|Rotator|MakeRotator 0.0 0.0 _doublespin) false false)
          (Transformation|SetRelativeRotation (Variables|Default|GetCube8) (Math|Rotator|MakeRotator 0.0 0.0 (* _doublespin -1.0)) false false))))
    (:B
      (Audio|PlaySoundatLocation "/Game/Game/Audio/SFX/drop-sound-effect-240899.drop-sound-effect-240899" (Transformation|GetActorLocation) "0, 0, 0" 1.0 1.0 0.0 0 0 0 0)
      (Transformation|SetActorRotation _light "-90.000000,0.000000,0.000000")
      (bind _doublespin_2 (Timeline|Timeline PlayFromStart)
        (:Update
          (Transformation|SetRelativeRotation (Variables|Default|GetCube2) (Math|Rotator|MakeRotator 0.0 0.0 (* _doublespin_2 -1.0)) false false)
          (Transformation|SetRelativeRotation (Variables|Default|GetCube8) (Math|Rotator|MakeRotator 0.0 0.0 _doublespin_2) false false))))))

(fn ConstructionScript)