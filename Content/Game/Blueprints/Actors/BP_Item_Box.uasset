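; BP_Item_Box is an interactable world pickup that adds its item to the interactor's inventory.
; The construction script sets the static mesh and physics simulation from ItemStruct.
; On Interact it passes ItemStruct to the interactor's BP_InventoryComponent, then plays the item's pickup sound and destroys itself on success, or plays a fallback sound on failure.
; GetInteractLocation returns the mesh's world location rather than the actor's.
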(event EventBeginPlay)

(event Collision|EventActorBeginOverlap
  (params (OtherActor :type Actor%20Object%20Reference)))

(event EventTick
  (params (DeltaSeconds :type Float%20%28single-precision%29)))

(event EventInteract
  (params (Interactor :type Actor%20Object%20Reference))
  (bind _issuccessful (Default|AddItemtoInventory (Actor|GetComponentbyClass Interactor "/Game/Game/Blueprints/Components/BP_InventoryComponent.BP_InventoryComponent_C") (Variables|Default|GetItemStruct)))
  (if _issuccessful
    (Audio|PlaySoundatLocation (.pickupsound (Variables|Default|GetItemStruct)) (Transformation|GetActorLocation) "0, 0, 0" 1.0 1.0 0.0 0 0 0 0)
    (Actor|DestroyActor)
    (else
      (Audio|PlaySoundatLocation "/Game/Game/Audio/SFX/electronic-hit-98242.electronic-hit-98242" (Transformation|GetActorLocation) "0, 0, 0" 1.0 1.0 0.0 0 0 0 0))))

(fn ConstructionScript
  (bind _itemstruct (Variables|Default|GetItemStruct))
  (Components|StaticMesh|SetStaticMesh (Variables|Default|GetStaticMesh) (.mesh _itemstruct))
  (Physics|SetSimulatePhysics (Variables|Default|GetStaticMesh) (.isphysical _itemstruct)))

(fn GetInteractLocation
  (return (Transformation|GetWorldLocation (Variables|Default|GetStaticMesh))))