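; Base dwarf actor that reacts to damage and death from its HealthComponent and can drop a pickup.
; Idle, damage and death timelines all drive one morph target, with dispatchers bound to stop the idle and damage animations.
; Hits play a randomized sound that rises in pitch as health falls, then resume idling.
; Death runs once, playing sound and animation before optionally spawning BP_PickupItem and destroying the actor.
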(event OnDeath(HealthComponent)
  (CallFunction|StopIdleLoop)
  (CallFunction|StopDamageTimeline)
  (Utilities|FlowControl|DoOnce false
    (:Completed
      (Class|BPIHealthComponent|MakeInvisible(Message) (Variables|Components|GetHealthComponent))
      (Audio|PlaySoundatLocation "/Game/Game/Audio/SFX/DwarfDeath.DwarfDeath" (Transformation|GetActorLocation) "0, 0, 0" 0.2 1.0 0.0 0 0 0 0)
      (bind _dies (Timeline|Die PlayFromStart)
        (:Update
          (Components|SkeletalMesh|SetMorphTarget (Variables|Components|GetDwarf) "Key_1" _dies true))
        (:Finished
          (if (Variables|Default|GetShouldDrop)
            (Game|SpawnActorfromClass "/Game/Game/Blueprints/Actors/BP_PickupItem.BP_PickupItem_C" (Transformation|GetActorTransform) "AlwaysSpawn" "MultiplyWithRoot" 0 0))
          (Actor|DestroyActor))))))

(event OnDamageTaken(HealthComponent)
  (bind _healthcomponent (Variables|Components|GetHealthComponent))
  (bind _maxhealth (Variables|/Game/Game/Blueprints/Components/HealthComponent.HealthComponent_C|GetMaxHealth _healthcomponent))
  (CallFunction|StopIdleLoop)
  (if (not (Variables|/Game/Game/Blueprints/Components/HealthComponent.HealthComponent_C|GetIsDead (Variables|Components|GetHealthComponent)))
    (Audio|PlaySoundatLocation "/Game/Game/Audio/SFX/a_clockwork_robot___-_AudioTrimmer_com_.a_clockwork_robot___-_AudioTrimmer_com_" (Transformation|GetActorLocation) "0, 0, 0" 0.2 (+ (* (Math|Float|NormalizetoRange (- _maxhealth (Variables|/Game/Game/Blueprints/Components/HealthComponent.HealthComponent_C|GetHealth _healthcomponent)) 0.0 _maxhealth) 2.0) (Math|Random|RandomFloatinRange -0.1 0.4)) 0.0 0 0 0 0)
    (bind _react (Timeline|TakeDamage PlayFromStart)
      (:Update
        (Components|SkeletalMesh|SetMorphTarget (Variables|Components|GetDwarf) "Key_1" _react true))
      (:Finished
        (CallFunction|IdleLoop)))))

(event Custom|IdleLoop
  (bind _idlemovement (Timeline|IdleMovement PlayFromStart)
    (:Update
      (Components|SkeletalMesh|SetMorphTarget (Variables|Components|GetDwarf) "Key_1" _idlemovement true))
    (:Finished
      (CallFunction|IdleLoop))))

(event Custom|StopIdleLoop
  (bind _idlemovement (Timeline|IdleMovement Stop)
    (:Update
      (Components|SkeletalMesh|SetMorphTarget (Variables|Components|GetDwarf) "Key_1" _idlemovement true))
    (:Finished
      (CallFunction|IdleLoop))))

(event Custom|StopDamageTimeline
  (bind _react (Timeline|TakeDamage Stop)
    (:Update
      (Components|SkeletalMesh|SetMorphTarget (Variables|Components|GetDwarf) "Key_1" _react true))
    (:Finished
      (CallFunction|IdleLoop))))

(event EventBeginPlay
  (EventDispatchers|BindEventtoStopIdleDispatcher (delegate Custom|StopIdleLoop))
  (EventDispatchers|BindEventtoStopDamageDispatcher (delegate Custom|StopDamageTimeline))
  (CallFunction|IdleLoop))

(event Collision|EventActorBeginOverlap
  (params (OtherActor :type Actor%20Object%20Reference)))

(event EventTick
  (params (DeltaSeconds :type Float%20%28single-precision%29)))

(fn ConstructionScript)