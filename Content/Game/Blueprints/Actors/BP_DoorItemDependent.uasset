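; BP_DoorItemDependent is an interactable door that stays locked until the player pays a toll of a specified item.
; Interacting charges the interactor's BP_InventoryComponent; success zeroes the toll, updates its text display and plays a cha-ching, while failure plays a latch sound.
; Once paid, interactions toggle the door, with one timeline played forward or reversed to rotate mesh and knob alongside a creak sound.
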(event Custom|OpenDoor
  (Variables|Default|SetisOpen true)
  (Audio|PlaySoundatLocation "/Game/Game/Audio/SFX/door-creaking-sound-effect-241381.door-creaking-sound-effect-241381" (Transformation|GetActorLocation) "0, 0, 0" 0.5 1.0 0.0 0 0 0 0)
  (bind (_direction _zrotation _knob) (Timeline|OpenDoorTimeline Play)
    (:Update
      (Transformation|SetRelativeRotation (Variables|Default|GetStaticMesh) (Math|Rotator|MakeRotator 0.0 0.0 _zrotation) false false)
      (Transformation|SetRelativeRotation (Variables|Default|GetCube2) (Math|Rotator|MakeRotator _knob 0.0 0.0) false false))))

(event Custom|CloseDoor
  (Variables|Default|SetisOpen false)
  (Audio|PlaySoundatLocation "/Game/Game/Audio/SFX/door-creaking-sound-effect-241381.door-creaking-sound-effect-241381" (Transformation|GetActorLocation) "0, 0, 0" 0.5 1.0 0.0 0 0 0 0)
  (bind (_direction _zrotation _knob) (Timeline|OpenDoorTimeline Reverse)
    (:Update
      (Transformation|SetRelativeRotation (Variables|Default|GetStaticMesh) (Math|Rotator|MakeRotator 0.0 0.0 _zrotation) false false)
      (Transformation|SetRelativeRotation (Variables|Default|GetCube2) (Math|Rotator|MakeRotator _knob 0.0 0.0) false false))))

(event EventInteract
  (params (Interactor :type Actor%20Object%20Reference))
  (if (<= (Variables|Default|Gettoll) 0)
    (if (Variables|Default|GetisOpen)
      (CallFunction|CloseDoor)
      (else
        (CallFunction|OpenDoor)))
    (else
      (bind _issuccessful (Default|AttempttoChargeAmount (Actor|GetComponentbyClass Interactor "/Game/Game/Blueprints/Components/BP_InventoryComponent.BP_InventoryComponent_C") (Variables|Default|Gettoll) (Variables|Default|GetItemToCharge)))
      (if _issuccessful
        (Variables|Default|Settoll 0)
        (Audio|PlaySoundatLocation "/Game/Game/Audio/SFX/cha-ching-7053.cha-ching-7053" (Transformation|GetActorLocation) "0, 0, 0" 1.0 1.0 0.0 0 0 0 0)
        (Rendering|Components|TextRender|SetText (Variables|Default|Get%20) (Utilities|Text|ToText(Integer) 0))
        (else
          (Audio|PlaySoundatLocation "/Game/Game/Audio/SFX/latch_02-108356.latch_02-108356" (Transformation|GetActorLocation) "0, 0, 0" 1.0 1.0 0.0 0 0 0 0))))))

(fn ConstructionScript
  (Rendering|Components|TextRender|SetText (Variables|Default|Get%20) (Utilities|Text|ToText(Integer) (Variables|Default|Gettoll))))

(fn GetInteractLocation
  (return (Transformation|GetWorldLocation (Variables|Default|GetCube2))))