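; Interactable zipline that carries the interactor along a spline, optionally behind a one-time item toll.
; Construction script looks up the toll item in DT_Items for the price display and tiles clamped-tangent spline meshes along the path.
; Interact charges the inventory component, clears the toll and starts the ride, or plays a latch sound on failure.
; The ride attaches the interactor, moves by length-scaled timeline and blocks saving until detach.
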(event Custom|UseZipline
  (bind _spline (Variables|Default|GetSpline))
  (bind _returnvalue (Spline|GetSplineLength _spline))
  (bind _asbp_custom_game_instance (Utilities|Casting|CastToBP_CustomGameInstance (Game|GetGameInstance)))
  (Variables|/Game/Game/Systems/BP_CustomGameInstance.BP_CustomGameInstance_C|SetisSaveingAllowed _asbp_custom_game_instance false)
  (Transformation|AttachComponentToComponent (stale EventInteract Interactor) (Variables|Default|GetCube2) "None" "SnapToTarget" "SnapToTarget" "KeepWorld" true)
  (Components|Timeline|SetPlayRate (Variables|Default|GetTimeline_1) (/ (Variables|Default|GetMoveSpeed) _returnvalue))
  (bind _newtrack_0 (Timeline|Timeline_1 PlayFromStart)
    (:Update
      (Transformation|SetWorldLocationAndRotation (Variables|Default|GetCube1) (.location (Spline|GetTransformatDistanceAlongSpline (Variables|Default|GetSpline) (Math|Float|Lerp 0.0 _returnvalue _newtrack_0) "World" false)) (.rotation (Spline|GetTransformatDistanceAlongSpline (Variables|Default|GetSpline) (Math|Float|Lerp 0.0 _returnvalue _newtrack_0) "World" false)) false false))
    (:Finished
      (Transformation|DetachFromActor (stale EventInteract Interactor) "KeepWorld" "KeepWorld" "KeepWorld")
      (bind _asbp_custom_game_instance_2 (Utilities|Casting|CastToBP_CustomGameInstance (Game|GetGameInstance)))
      (Variables|/Game/Game/Systems/BP_CustomGameInstance.BP_CustomGameInstance_C|SetisSaveingAllowed _asbp_custom_game_instance_2 true))))

(event EventInteract
  (params (Interactor :type Actor%20Object%20Reference))
  (if (<= (Variables|Default|Gettoll) 0)
    (CallFunction|UseZipline)
    (else
      (bind _issuccessful (Default|AttempttoChargeAmount (Actor|GetComponentbyClass Interactor "/Game/Game/Blueprints/Components/BP_InventoryComponent.BP_InventoryComponent_C") (Variables|Default|Gettoll) (Variables|Default|GetItemToCharge)))
      (if _issuccessful
        (Variables|Default|Settoll 0)
        (Audio|PlaySoundatLocation (.usesound (Variables|Default|GetItemToCharge)) (Transformation|GetActorLocation) "0, 0, 0" 1.0 1.0 0.0 0 0 0 0)
        (Rendering|SetVisibility (Variables|Default|GetText) false false)
        (Components|StaticMesh|SetStaticMesh (Variables|Default|GetStaticMesh) 0)
        (CallFunction|UseZipline)
        (else
          (Audio|PlaySoundatLocation "/Game/Game/Audio/SFX/latch_02-108356.latch_02-108356" (Transformation|GetActorLocation) "0, 0, 0" 1.0 1.0 0.0 0 0 0 0))))))

(fn ConstructionScript
  (bind _text (Variables|Default|GetText))
  (Utilities|FlowControl|Sequence
    (:then_0
      (bind _returnvalue (Utilities|GetDataTableRow "/Game/Game/Systems/Inventory/DT_Items.DT_Items" (Variables|Default|GetRow%20Name))
        (:then
          (Variables|Default|SetItemToCharge _returnvalue)
          (if (> (Variables|Default|Gettoll) 0)
            (Rendering|Components|TextRender|SetText _text (Utilities|Text|ToText(Integer) (Variables|Default|Gettoll)))
            (Components|StaticMesh|SetStaticMesh (Variables|Default|GetStaticMesh) (.mesh (Variables|Default|GetItemToCharge)))
            (else
              (Rendering|SetVisibility _text false false))))))
    (:then_1
      (bind _output_get (Variables|Default|SetSectionLength (.x (.boxextent (StaticMesh|GetBounds (Variables|Default|GetSplineMesh))))))
      (for _index (range 0 (Math|Float|Truncate (/ (Spline|GetSplineLength (Variables|Default|GetSpline)) _output_get)))
        (Variables|Default|SetIndex _index)
        (bind _returnvalue_2 (AddComponent|AddSplineMeshComponent false (Transformation|GetActorTransform)))
        (Components|StaticMesh|SetStaticMesh _returnvalue_2 (Variables|Default|GetSplineMesh))
        (SplineMesh|SetForwardAxis _returnvalue_2 "X" true)
        (bind (_position _tangent) (CallFunction|GetStartPos/Tangent (Variables|Default|GetIndex)))
        (bind (_position_2 _tangent_2) (CallFunction|GetEndPos/Tangent (Variables|Default|GetIndex)))
        (SplineMesh|SetStartandEnd _returnvalue_2 _position _tangent _position_2 _tangent_2 true :!class /Script/Engine.SplineMeshComponent)
        (Collision|SetCollisionEnabled _returnvalue_2 "NoCollision")))))

(fn GetStartPos/Tangent
  (params (Index :type Integer))
  (bind _spline (Variables|Default|GetSpline))
  (bind _sectionlength (Variables|Default|GetSectionLength))
  (bind _returnvalue (* _sectionlength Index))
  (return (Spline|GetLocationatDistanceAlongSpline _spline _returnvalue "Local") (Math|Vector|ClampVectorSize (Spline|GetTangentatDistanceAlongSpline _spline _returnvalue "Local") 0.0 _sectionlength)))

(fn GetEndPos/Tangent
  (params (Index :type Integer))
  (bind _returnvalue (+ Index 1))
  (bind _spline (Variables|Default|GetSpline))
  (bind _sectionlength (Variables|Default|GetSectionLength))
  (bind _returnvalue_2 (* _sectionlength _returnvalue))
  (return (Spline|GetLocationatDistanceAlongSpline _spline _returnvalue_2 "Local") (Math|Vector|ClampVectorSize (Spline|GetTangentatDistanceAlongSpline _spline _returnvalue_2 "Local") 0.0 _sectionlength)))

(fn CountasInteractable
  (return (Variables|Default|GetIsInteractable)))

(fn GetInteractLocation
  (return (Transformation|GetWorldLocation (Variables|Default|GetBox))))