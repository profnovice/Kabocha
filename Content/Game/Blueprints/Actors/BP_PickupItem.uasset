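; BP_PickupItem is an interactable pickup actor that removes itself from the world when used.
; Its Interact event prints an "added to inventory" message naming the item and interactor, plays a coin-bag sound at its location, then destroys the actor.
; The inventory step is only that printed message; no item data is passed to the interactor.
; GetInteractLocation reports the actor's own location as the interaction point.
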(event EventInteract
  (params (Interactor :type Actor%20Object%20Reference))
  (Development|PrintString (Utilities|String|ToString(Text) (Utilities|Text|FormatText "added {itemName} to inventory of {actorName}" (Utilities|GetDisplayName self) (Utilities|GetDisplayName Interactor))))
  (Audio|PlaySoundatLocation "/Game/Game/Audio/SFX/coin-and-money-bag-3-185264.coin-and-money-bag-3-185264" (Transformation|GetActorLocation) "0, 0, 0" 1.0 1.0 0.0 0 0 0 0)
  (Actor|DestroyActor))

(fn ConstructionScript)

(fn GetInteractLocation
  (return (Transformation|GetActorLocation)))