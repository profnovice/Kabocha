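; Interactable lever switch that toggles up or down and triggers a linked actor.
; Interact plays a sound and runs one of two timelines to rotate the lever arm, then sends an Interact message to ActorToAffect when the swing finishes.
; The construction script poses the lever from StartAsUp, and SwitchOnlyOnce makes it non-interactable after first use.
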(event EventBeginPlay)

(event Collision|EventActorBeginOverlap
  (params (OtherActor :type Actor%20Object%20Reference)))

(event EventTick
  (params (DeltaSeconds :type Float%20%28single-precision%29)))

(event EventInteract
  (params (Interactor :type Actor%20Object%20Reference))
  (if (Variables|Default|GetSwitchOnlyOnce)
    (Utilities|FlowControl|DoOnce false
      (:Completed
        (Variables|Default|SetIsInteractable false))))
  (Audio|PlaySoundatLocation (Variables|Default|GetSound) (Transformation|GetActorLocation) "0, 0, 0" 1.0 1.0 0.0 0 0 0 0)
  (if (Variables|Default|GetIsUp)
    (bind _newtrack_0 (Timeline|Timeline_0 PlayFromStart)
      (:Update
        (Transformation|SetRelativeRotation (Variables|Default|GetLeverArm) (Math|Rotator|MakeRotator (* _newtrack_0 -1.0) 0.0 0.0) false false)
        (Variables|Default|SetIsUp false))
      (:Finished
        (Class|BPIInteractable|Interact(Message) (Variables|Default|GetActorToAffect) self :!label _label)))
    (else
      (bind _newtrack_0_2 (Timeline|Timeline PlayFromStart)
        (:Update
          (Transformation|SetRelativeRotation (Variables|Default|GetLeverArm) (Math|Rotator|MakeRotator _newtrack_0_2 0.0 0.0) false false)
          (Variables|Default|SetIsUp true))
        (:Finished
          (goto _label))))))

(fn ConstructionScript
  (bind _leverarm (Variables|Default|GetLeverArm))
  (Variables|Default|SetIsUp (Variables|Default|GetStartAsUp))
  (if (Variables|Default|GetStartAsUp)
    (Transformation|SetRelativeRotation _leverarm "0.000000,0.000000,-70.000000" false false)
    (else
      (Transformation|SetRelativeRotation _leverarm "0.000000,0.000000,70.000000" false false))))

(fn CountasInteractable
  (return (Variables|Default|GetIsInteractable)))

(fn GetInteractLocation
  (return (Transformation|GetActorLocation)))