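; Interactable lever switch that flips between up and down and sends an interact message to a linked actor.
; Interact plays a sound and a timeline that rotates the lever and updates its state, messaging ActorToAffect on finish; SwitchOnlyOnce disables further interaction.
; The construction script poses the lever from StartAsUp.
; State and interactability save per level by object name, and loading restores the lever pose.
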(event Custom|UpdatePhysicalState
  (bind _leverarm (Variables|Default|GetLeverArm))
  (if (Utilities|Enum|Equal(Enum) (Variables|Default|GetInteractable%20State) "NewEnumerator2")
    (Transformation|SetRelativeRotation _leverarm "0.000000,0.000000,-70.000000" false false)
    (else
      (Transformation|SetRelativeRotation _leverarm "0.000000,0.000000,70.000000" false false))))

(event EventBeginPlay
  (Class|BPIPersistance|RequestLoad(Message) (Game|GetGameInstance) self))

(event Collision|EventActorBeginOverlap
  (params (OtherActor :type Actor%20Object%20Reference)))

(event EventTick
  (params (DeltaSeconds :type Float%20%28single-precision%29)))

(event EventInteract
  (params (Interactor :type Actor%20Object%20Reference))
  (if (Variables|Default|GetSwitchOnlyOnce)
    (Utilities|FlowControl|DoOnce false
      (:Completed
        (Variables|Default|SetIsInteractable false))))
  (Audio|PlaySoundatLocation (Variables|Default|GetSound) (Transformation|GetActorLocation) "0, 0, 0" 1.0 1.0 0.0 0 0 0 0)
  (if (Utilities|Enum|Equal(Enum) (Variables|Default|GetInteractable%20State) "NewEnumerator2")
    (bind _newtrack_0 (Timeline|Timeline_0 PlayFromStart)
      (:Update
        (Transformation|SetRelativeRotation (Variables|Default|GetLeverArm) (Math|Rotator|MakeRotator (* _newtrack_0 -1.0) 0.0 0.0) false false)
        (Variables|Default|SetIsUp false)
        (Variables|Default|SetInteractable%20State "NewEnumerator3"))
      (:Finished
        (Class|BPIInteractable|Interact(Message) (Variables|Default|GetActorToAffect) self :!label _label)))
    (else
      (bind _newtrack_0_2 (Timeline|Timeline PlayFromStart)
        (:Update
          (Transformation|SetRelativeRotation (Variables|Default|GetLeverArm) (Math|Rotator|MakeRotator _newtrack_0_2 0.0 0.0) false false)
          (Variables|Default|SetIsUp true)
          (Variables|Default|SetInteractable%20State "NewEnumerator2"))
        (:Finished
          (goto _label))))))

(event EventLoadObjectData
  (params (SaveGameRef :type BP%20Save%20Game%20Object%20Reference) (LevelDataRef :type Integer))
  (bind _self self)
  (bind _levelstates (Variables|/Game/Game/SaveGame/BP_SaveGame.BP_SaveGame_C|GetLevelStates SaveGameRef))
  (bind _returnvalue (Utilities|GetObjectName _self))
  (bind _output (Utilities|Array|Get(acopy) _levelstates LevelDataRef))
  (bind _returnvalue_2 (Utilities|String|StringToName _returnvalue))
  (bind (_value _returnvalue_3) (Utilities|Map|Find (.staticinteractablesdata _output) _returnvalue_2))
  (bind (_state _isinteractable) (Utilities|Struct|BreakST_InteractableData _value))
  (if (.isvalid _output)
    (if _returnvalue_3
      (Variables|Default|SetInteractable%20State _state)
      (Variables|Default|SetIsInteractable _isinteractable)
      (CallFunction|UpdatePhysicalState))))

(event EventSaveObjectData
  (params (SaveGameRef :type BP%20Save%20Game%20Object%20Reference) (LevelDataRef :type Integer))
  (Utilities|Map|Add (.staticinteractablesdata (Utilities|Array|Get(acopy) (Variables|/Game/Game/SaveGame/BP_SaveGame.BP_SaveGame_C|GetLevelStates SaveGameRef) LevelDataRef)) (Utilities|String|StringToName (Utilities|GetObjectName self)) (Utilities|Struct|MakeST_InteractableData (Variables|Default|GetInteractable%20State) (Variables|Default|GetIsInteractable))))

(fn ConstructionScript
  (bind _leverarm (Variables|Default|GetLeverArm))
  (Variables|Default|SetIsUp (Variables|Default|GetStartAsUp))
  (if (Variables|Default|GetStartAsUp)
    (Variables|Default|SetInteractable%20State "NewEnumerator2")
    (Transformation|SetRelativeRotation _leverarm "0.000000,0.000000,-70.000000" false false)
    (else
      (Transformation|SetRelativeRotation _leverarm "0.000000,0.000000,70.000000" false false))))

(fn CountasInteractable
  (return (Variables|Default|GetIsInteractable)))

(fn GetInteractLocation
  (return (Transformation|GetActorLocation)))