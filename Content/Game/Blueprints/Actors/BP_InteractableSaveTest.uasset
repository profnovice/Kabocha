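; Test interactable actor that toggles between two states and persists its state through the save system.
; Interact flips InteractableState, then swaps the Closed and OPEN components between the TopArrow and BottomArrow transforms.
; BeginPlay requests a load from the GameInstance; save and load handlers store and restore the state in the level's StaticInteractablesData map, keyed by object name.
; The construction script resets it to the default state.
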(event Custom|UpdatePhysicalState
  (if (Utilities|Enum|Equal(Enum) (Variables|Default|GetInteractableState) "NewEnumerator0")
    (Transformation|SetRelativeTransform (Variables|Default|GetClosed) (Transformation|GetRelativeTransform (Variables|Default|GetTopArrow)) false true)
    (Transformation|SetRelativeTransform (Variables|Default|GetOPEN) (Transformation|GetRelativeTransform (Variables|Default|GetBottomArrow)) false true)
    (else
      (Transformation|SetRelativeTransform (Variables|Default|GetOPEN) (Transformation|GetRelativeTransform (Variables|Default|GetTopArrow)) false true)
      (Transformation|SetRelativeTransform (Variables|Default|GetClosed) (Transformation|GetRelativeTransform (Variables|Default|GetBottomArrow)) false true))))

(event EventBeginPlay
  (Class|BPIPersistance|RequestLoad(Message) (Game|GetGameInstance) self))

(event Collision|EventActorBeginOverlap
  (params (OtherActor :type Actor%20Object%20Reference)))

(event EventTick
  (params (DeltaSeconds :type Float%20%28single-precision%29)))

(event EventInteract
  (params (Interactor :type Actor%20Object%20Reference))
  (if (Utilities|Enum|Equal(Enum) (Variables|Default|GetInteractableState) "NewEnumerator0")
    (Variables|Default|SetInteractableState "NewEnumerator1")
    (else
      (Variables|Default|SetInteractableState "NewEnumerator0")))
  (CallFunction|UpdatePhysicalState))

(event EventLoadObjectData
  (params (SaveGameRef :type BP%20Save%20Game%20Object%20Reference) (LevelDataRef :type Integer))
  (bind _self self)
  (bind _levelstates (Variables|/Game/Game/SaveGame/BP_SaveGame.BP_SaveGame_C|GetLevelStates SaveGameRef))
  (bind _returnvalue (Utilities|GetObjectName _self))
  (bind _output (Utilities|Array|Get(acopy) _levelstates LevelDataRef))
  (bind _returnvalue_2 (Utilities|String|StringToName _returnvalue))
  (bind (_value _returnvalue_3) (Utilities|Map|Find (.staticinteractablesdata _output) _returnvalue_2))
  (if (.isvalid _output)
    (if _returnvalue_3
      (Variables|Default|SetInteractableState (Utilities|Struct|BreakST_InteractableData _value))
      (CallFunction|UpdatePhysicalState))))

(event EventSaveObjectData
  (params (SaveGameRef :type BP%20Save%20Game%20Object%20Reference) (LevelDataRef :type Integer))
  (Utilities|Map|Add (.staticinteractablesdata (Utilities|Array|Get(acopy) (Variables|/Game/Game/SaveGame/BP_SaveGame.BP_SaveGame_C|GetLevelStates SaveGameRef) LevelDataRef)) (Utilities|String|StringToName (Utilities|GetObjectName self)) (Utilities|Struct|MakeST_InteractableData (Variables|Default|GetInteractableState))))

(fn ConstructionScript
  (Variables|Default|SetInteractableState "NewEnumerator0")
  (CallFunction|UpdatePhysicalState))

(fn CountasInteractable
  (return true))

(fn GetInteractLocation
  (return (Transformation|GetActorLocation)))