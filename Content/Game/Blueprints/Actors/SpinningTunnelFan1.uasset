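; Interactable tunnel fan that toggles between spinning and stopped, with its initial state set by ShouldSpin.
; A timeline replays itself to loop the rotation while on, with separate timelines easing it down and, played in reverse, spinning it back up.
; The fan's looping audio pauses and resumes with the state.
; State and interactability persist per level in the save game, keyed by object name, with loading requested through the game instance.
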(event Custom|Spin
  (bind _newtrack_0 (Timeline|Timeline PlayFromStart)
    (:Update
      (Transformation|SetRelativeRotation (Variables|Default|GetTunnnelCircleFan) (Math|Rotator|MakeRotator 0.0 _newtrack_0 0.0) false false))
    (:Finished
      (if (Utilities|Enum|Equal(Enum) (Variables|Default|GetInteractable%20State) "NewEnumerator0")
        (CallFunction|Spin)
        (else
          (bind _newtrack_0_2 (Timeline|Timeline_0 PlayFromStart)
            (:Update
              (Transformation|SetRelativeRotation (Variables|Default|GetTunnnelCircleFan) (Math|Rotator|MakeRotator 0.0 _newtrack_0_2 0.0) false false)
              (Class|AudioComponent|SetPaused (Variables|Default|GetAudio) true))))))))

(event Custom|PlaySound)

(event Custom|UpdatePhysicalState
  (bind _audio (Variables|Default|GetAudio))
  (if (Utilities|Enum|Equal(Enum) (Variables|Default|GetInteractable%20State) "NewEnumerator0")
    (Class|AudioComponent|SetPaused _audio false)
    (Audio|Components|Audio|Play _audio 0.0)
    (CallFunction|Spin)))

(event EventBeginPlay
  (if (Variables|Default|GetShouldSpin)
    (Variables|Default|SetInteractable%20State "NewEnumerator0")
    (else
      (Variables|Default|SetInteractable%20State "NewEnumerator1")))
  (Class|BPIPersistance|RequestLoad(Message) (Game|GetGameInstance) self)
  (Audio|Components|Audio|SetSound (Variables|Default|GetAudio) "/Game/Game/Audio/SFX/large-fan-38268.large-fan-38268")
  (CallFunction|UpdatePhysicalState))

(event EventInteract
  (params (Interactor :type Actor%20Object%20Reference))
  (bind _audio (Variables|Default|GetAudio))
  (if (Utilities|Enum|Equal(Enum) (Variables|Default|GetInteractable%20State) "NewEnumerator0")
    (Variables|Default|SetInteractable%20State "NewEnumerator1")
    (else
      (Variables|Default|SetInteractable%20State "NewEnumerator0")
      (Class|AudioComponent|SetPaused _audio false)
      (Audio|Components|Audio|Play _audio 0.0)
      (bind _newtrack_0 (Timeline|Timeline_1 ReverseFromEnd)
        (:Update
          (Transformation|SetRelativeRotation (Variables|Default|GetTunnnelCircleFan) (Math|Rotator|MakeRotator 0.0 (* _newtrack_0 -1.0) 0.0) false false))
        (:Finished
          (CallFunction|Spin))))))

(event EventLoadObjectData
  (params (SaveGameRef :type BP%20Save%20Game%20Object%20Reference) (LevelDataRef :type Integer))
  (bind _self self)
  (bind _levelstates (Variables|/Game/Game/SaveGame/BP_SaveGame.BP_SaveGame_C|GetLevelStates SaveGameRef))
  (bind _returnvalue (Utilities|GetObjectName _self))
  (bind _output (Utilities|Array|Get(acopy) _levelstates LevelDataRef))
  (bind _returnvalue_2 (Utilities|String|StringToName _returnvalue))
  (bind (_value _returnvalue_3) (Utilities|Map|Find (.staticinteractablesdata _output) _returnvalue_2))
  (bind (_state _isinteractable) (Utilities|Struct|BreakST_InteractableData _value))
  (if (.isvalid _output)
    (if _returnvalue_3
      (Variables|Default|SetInteractable%20State _state)
      (Variables|Default|SetIsInteractable _isinteractable)
      (CallFunction|UpdatePhysicalState))))

(event EventSaveObjectData
  (params (SaveGameRef :type BP%20Save%20Game%20Object%20Reference) (LevelDataRef :type Integer))
  (Utilities|Map|Add (.staticinteractablesdata (Utilities|Array|Get(acopy) (Variables|/Game/Game/SaveGame/BP_SaveGame.BP_SaveGame_C|GetLevelStates SaveGameRef) LevelDataRef)) (Utilities|String|StringToName (Utilities|GetObjectName self)) (Utilities|Struct|MakeST_InteractableData (Variables|Default|GetInteractable%20State) (Variables|Default|GetIsInteractable))))

(fn ConstructionScript)

(fn CountasInteractable
  (return (Variables|Default|GetisInteractable)))

(fn GetInteractLocation
  (return (Transformation|GetWorldLocation (Variables|Default|GetBox))))