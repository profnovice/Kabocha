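; BP_Cake is an interactable actor that saves the game and then opens a level.
; On interaction it binds to the custom game instance's game-saved event and requests a save, deferring the level load until that callback fires.
; It reports itself as interactable at its own location.
; Disconnected leftover pickup logic would print an inventory message, play a coin sound and destroy the actor, but never runs.
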(event Custom|Saved
  (params (SaveGameRef :type BP%20Save%20Game%20Object%20Reference))
  (Game|OpenLevel(byObjectReference) (Variables|Default|GetLevel)))

(event EventInteract
  (params (Interactor :type Actor%20Object%20Reference))
  (bind _asbp_custom_game_instance (Utilities|Casting|CastToBP_CustomGameInstance (Game|GetGameInstance)))
  (EventDispatchers|BindEventtoGameIsSaved _asbp_custom_game_instance (delegate Custom|Saved))
  (Class|BPIPersistance|RequestSave(Message) _asbp_custom_game_instance false))

(fn ConstructionScript)

(fn CountasInteractable
  (return true))

(fn GetInteractLocation
  (return (Transformation|GetActorLocation)))