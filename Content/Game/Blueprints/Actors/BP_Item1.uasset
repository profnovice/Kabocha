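; BP_Item1 is an interactable item pickup that can be collected into an actor's inventory.
; The Construction Script fills ItemStruct from a DT_Items row when RowName is set, applies mesh and physics, and line-traces non-physical items down to the surface below.
; Interact passes the struct to the interactor's BP_InventoryComponent, playing the pickup sound and destroying itself on success, or a fallback sound otherwise.
; BeginPlay calls HeatBeat, which is empty.
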(event Custom|HeatBeat)

(event EventBeginPlay
  (CallFunction|HeatBeat))

(event Collision|EventActorBeginOverlap
  (params (OtherActor :type Actor%20Object%20Reference)))

(event EventTick
  (params (DeltaSeconds :type Float%20%28single-precision%29)))

(event EventInteract
  (params (Interactor :type Actor%20Object%20Reference))
  (bind _issuccessful (Default|AddItemtoInventory (Actor|GetComponentbyClass Interactor "/Game/Game/Blueprints/Components/BP_InventoryComponent.BP_InventoryComponent_C") (Variables|Default|GetItemStruct)))
  (if _issuccessful
    (Audio|PlaySoundatLocation (.pickupsound (Variables|Default|GetItemStruct)) (Transformation|GetActorLocation) "0, 0, 0" 1.0 1.0 0.0 0 0 0 0)
    (Actor|DestroyActor)
    (else
      (Audio|PlaySoundatLocation "/Game/Game/Audio/SFX/electronic-hit-98242.electronic-hit-98242" (Transformation|GetActorLocation) "0, 0, 0" 1.0 1.0 0.0 0 0 0 0))))

(fn ConstructionScript
  (bind _returnvalue (Transformation|GetActorLocation))
  (bind _row_name (Variables|Default|GetRow%20Name))
  (bind (_x _y _z) (Math|Vector|BreakVector _returnvalue))
  (bind (_x_2 _y_2 _z_2) (Math|Vector|BreakVector _returnvalue))
  (if (== _row_name "Null")
    _
    (else
      (bind _returnvalue_2 (Utilities|GetDataTableRow "/Game/Game/Systems/Inventory/DT_Items.DT_Items" _row_name)
        (:then
          (Variables|Default|SetItemStruct (Utilities|Struct|MakeST_Item (.Name (Utilities|Struct|BreakST_Item _returnvalue_2)) (.Stackable (Utilities|Struct|BreakST_Item _returnvalue_2)) (Variables|Default|GetQuanity) (.Thumbnail (Utilities|Struct|BreakST_Item _returnvalue_2)) (.Mesh (Utilities|Struct|BreakST_Item _returnvalue_2)) (.PickupSound (Utilities|Struct|BreakST_Item _returnvalue_2)) (.MaxCarryQuantity (Utilities|Struct|BreakST_Item _returnvalue_2)) (.IsPhysical (Utilities|Struct|BreakST_Item _returnvalue_2)) (.DropSound (Utilities|Struct|BreakST_Item _returnvalue_2))))))))
  (Components|StaticMesh|SetStaticMesh (Variables|Default|GetStaticMesh) (.mesh (Variables|Default|GetItemStruct)))
  (Physics|SetSimulatePhysics (Variables|Default|GetStaticMesh) (.isphysical (Variables|Default|GetItemStruct)))
  (if (not (.isphysical (Variables|Default|GetItemStruct)))
    (bind _outhit (Collision|LineTraceByChannel (Math|Vector|MakeVector _x_2 _y_2 (+ _z_2 5e+01)) (Math|Vector|MakeVector _x _y (- _z 1e+03)) "TraceTypeQuery1" false (Utilities|Array|MakeArray 0) "None"))
    (Transformation|SetActorLocation (.Location (Collision|BreakHitResult _outhit)) false true)))

(fn CountasInteractable
  (return true))

(fn GetInteractLocation
  (return (Transformation|GetWorldLocation (Variables|Default|GetStaticMesh))))