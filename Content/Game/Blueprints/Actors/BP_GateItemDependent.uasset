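; Interactable double gate that stays locked until the interactor pays an item toll from its inventory component, then opens or closes on later interactions.
; Construction script looks up the item in DT_Items to show the toll count and item mesh, both cleared once paid.
; One timeline swings both leaves in opposite directions, reversing to close, and OpenOnlyOnce disables interaction after the first toll-free use.
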(event Custom|OpenDoor
  (Variables|Default|SetisOpen true)
  (Audio|PlaySoundatLocation "/Game/Game/Audio/SFX/gate-close-and-rattle-42494.gate-close-and-rattle-42494" (Transformation|GetActorLocation) "0, 0, 0" 0.5 1.0 0.0 0 0 0 0)
  (bind _zrotation (Timeline|OpenDoorTimeline Play)
    (:Update
      (Transformation|SetRelativeRotation (Variables|Default|GetGate) (Math|Rotator|MakeRotator 0.0 0.0 _zrotation) false false)
      (Transformation|SetRelativeRotation (Variables|Default|GetGate1) (Math|Rotator|MakeRotator 0.0 0.0 (* _zrotation -1.0)) false false))))

(event Custom|CloseDoor
  (Variables|Default|SetisOpen false)
  (Audio|PlaySoundatLocation "/Game/Game/Audio/SFX/gate-close-and-rattle-42494.gate-close-and-rattle-42494" (Transformation|GetActorLocation) "0, 0, 0" 0.5 1.0 0.0 0 0 0 0)
  (bind _zrotation (Timeline|OpenDoorTimeline Reverse)
    (:Update
      (Transformation|SetRelativeRotation (Variables|Default|GetGate) (Math|Rotator|MakeRotator 0.0 0.0 _zrotation) false false)
      (Transformation|SetRelativeRotation (Variables|Default|GetGate1) (Math|Rotator|MakeRotator 0.0 0.0 (* _zrotation -1.0)) false false))))

(event EventInteract
  (params (Interactor :type Actor%20Object%20Reference))
  (if (<= (Variables|Default|Gettoll) 0)
    (if (Variables|Default|GetOpenOnlyOnce)
      (Utilities|FlowControl|DoOnce false
        (:Completed
          (Variables|Default|SetIsInteractable false))))
    (if (Variables|Default|GetisOpen)
      (CallFunction|CloseDoor)
      (else
        (CallFunction|OpenDoor)))
    (else
      (bind _issuccessful (Default|AttempttoChargeAmount (Actor|GetComponentbyClass Interactor "/Game/Game/Blueprints/Components/BP_InventoryComponent.BP_InventoryComponent_C") (Variables|Default|Gettoll) (Variables|Default|GetItemToCharge)))
      (if _issuccessful
        (Variables|Default|Settoll 0)
        (Audio|PlaySoundatLocation (.usesound (Variables|Default|GetItemToCharge)) (Transformation|GetActorLocation) "0, 0, 0" 1.0 1.0 0.0 0 0 0 0)
        (Rendering|SetVisibility (Variables|Default|GetText) false false)
        (Components|StaticMesh|SetStaticMesh (Variables|Default|GetStaticMesh) 0)
        (else
          (Audio|PlaySoundatLocation "/Game/Game/Audio/SFX/latch_02-108356.latch_02-108356" (Transformation|GetActorLocation) "0, 0, 0" 1.0 1.0 0.0 0 0 0 0))))))

(fn ConstructionScript
  (bind _text (Variables|Default|GetText))
  (bind _returnvalue (Utilities|GetDataTableRow "/Game/Game/Systems/Inventory/DT_Items.DT_Items" (Variables|Default|GetRow%20Name))
    (:then
      (Variables|Default|SetItemToCharge _returnvalue)
      (if (> (Variables|Default|Gettoll) 0)
        (Rendering|Components|TextRender|SetText _text (Utilities|Text|ToText(Integer) (Variables|Default|Gettoll)))
        (Components|StaticMesh|SetStaticMesh (Variables|Default|GetStaticMesh) (.mesh (Variables|Default|GetItemToCharge)))
        (else
          (Rendering|SetVisibility _text false false))))))

(fn CountasInteractable
  (return (Variables|Default|GetIsInteractable)))

(fn GetInteractLocation
  (return (Transformation|GetWorldLocation (Variables|Default|GetBox))))