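; Interactable double gate that stays shut until the interactor pays a toll in a configured item.
; Construction shows the DT_Items mesh and toll count; Interact charges the interactor's inventory component, clearing both on success.
; Later interactions toggle a timeline swinging both leaves in mirror, optionally only once.
; State, interactability and remaining toll save per level by object name; load is requested on BeginPlay and snaps the gate's pose.
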(event Custom|OpenDoor
  (Variables|Default|SetInteractable%20State "NewEnumerator1")
  (Audio|PlaySoundatLocation "/Game/Game/Audio/SFX/gate-close-and-rattle-42494.gate-close-and-rattle-42494" (Transformation|GetActorLocation) "0, 0, 0" 0.5 1.0 0.0 0 0 0 0)
  (bind _zrotation (Timeline|OpenDoorTimeline PlayFromStart)
    (:Update
      (Transformation|SetRelativeRotation (Variables|Default|GetGate) (Math|Rotator|MakeRotator 0.0 0.0 _zrotation) false false)
      (Transformation|SetRelativeRotation (Variables|Default|GetGate1) (Math|Rotator|MakeRotator 0.0 0.0 (* _zrotation -1.0)) false false))))

(event Custom|CloseDoor
  (Variables|Default|SetInteractable%20State "NewEnumerator0")
  (Audio|PlaySoundatLocation "/Game/Game/Audio/SFX/gate-close-and-rattle-42494.gate-close-and-rattle-42494" (Transformation|GetActorLocation) "0, 0, 0" 0.5 1.0 0.0 0 0 0 0)
  (bind _zrotation (Timeline|OpenDoorTimeline ReverseFromEnd)
    (:Update
      (Transformation|SetRelativeRotation (Variables|Default|GetGate) (Math|Rotator|MakeRotator 0.0 0.0 _zrotation) false false)
      (Transformation|SetRelativeRotation (Variables|Default|GetGate1) (Math|Rotator|MakeRotator 0.0 0.0 (* _zrotation -1.0)) false false))))

(event Custom|UpdatePhysicalState
  (bind _returnvalue (Math|Float|MakeLiteralFloat -9e+01))
  (bind _returnvalue_2 (Math|Float|MakeLiteralFloat 0.0))
  (if (<= (Variables|Default|Gettoll) 0)
    (Rendering|SetVisibility (Variables|Default|GetText) false false)
    (Components|StaticMesh|SetStaticMesh (Variables|Default|GetStaticMesh) 0))
  (if (Utilities|Enum|Equal(Enum) (Variables|Default|GetInteractable%20State) "NewEnumerator1")
    (Transformation|SetRelativeRotation (Variables|Default|GetGate) (Math|Rotator|MakeRotator 0.0 0.0 _returnvalue_2) false false)
    (Transformation|SetRelativeRotation (Variables|Default|GetGate1) (Math|Rotator|MakeRotator 0.0 0.0 (* _returnvalue_2 -1.0)) false false)
    (else
      (Transformation|SetRelativeRotation (Variables|Default|GetGate) (Math|Rotator|MakeRotator 0.0 0.0 _returnvalue) false false)
      (Transformation|SetRelativeRotation (Variables|Default|GetGate1) (Math|Rotator|MakeRotator 0.0 0.0 (* _returnvalue -1.0)) false false))))

(event EventBeginPlay
  (Class|BPIPersistance|RequestLoad(Message) (Game|GetGameInstance) self))

(event EventInteract
  (params (Interactor :type Actor%20Object%20Reference))
  (if (<= (Variables|Default|Gettoll) 0)
    (if (Variables|Default|GetOpenOnlyOnce)
      (Utilities|FlowControl|DoOnce false
        (:Completed
          (Variables|Default|SetIsInteractable false))))
    (if (Utilities|Enum|Equal(Enum) (Variables|Default|GetInteractable%20State) "NewEnumerator1")
      (CallFunction|CloseDoor)
      (else
        (CallFunction|OpenDoor)))
    (else
      (bind _issuccessful (Default|AttempttoChargeAmount (Actor|GetComponentbyClass Interactor "/Game/Game/Blueprints/Components/BP_InventoryComponent.BP_InventoryComponent_C") (Variables|Default|Gettoll) (Variables|Default|GetItemToCharge)))
      (if _issuccessful
        (Variables|Default|Settoll 0)
        (Audio|PlaySoundatLocation (.usesound (Variables|Default|GetItemToCharge)) (Transformation|GetActorLocation) "0, 0, 0" 1.0 1.0 0.0 0 0 0 0)
        (Rendering|SetVisibility (Variables|Default|GetText) false false)
        (Components|StaticMesh|SetStaticMesh (Variables|Default|GetStaticMesh) 0)
        (else
          (Audio|PlaySoundatLocation "/Game/Game/Audio/SFX/latch_02-108356.latch_02-108356" (Transformation|GetActorLocation) "0, 0, 0" 1.0 1.0 0.0 0 0 0 0))))))

(event EventLoadObjectData
  (params (SaveGameRef :type BP%20Save%20Game%20Object%20Reference) (LevelDataRef :type Integer))
  (bind _self self)
  (bind _levelstates (Variables|/Game/Game/SaveGame/BP_SaveGame.BP_SaveGame_C|GetLevelStates SaveGameRef))
  (bind _returnvalue (Utilities|GetObjectName _self))
  (bind _output (Utilities|Array|Get(acopy) _levelstates LevelDataRef))
  (bind _returnvalue_2 (Utilities|String|StringToName _returnvalue))
  (bind (_value _returnvalue_3) (Utilities|Map|Find (.staticinteractablesdata _output) _returnvalue_2))
  (bind (_state _isinteractable _toll) (Utilities|Struct|BreakST_InteractableData _value))
  (if (.isvalid _output)
    (if _returnvalue_3
      (Variables|Default|SetInteractable%20State _state)
      (Variables|Default|SetIsInteractable _isinteractable)
      (Variables|Default|Settoll _toll)
      (CallFunction|UpdatePhysicalState))))

(event EventSaveObjectData
  (params (SaveGameRef :type BP%20Save%20Game%20Object%20Reference) (LevelDataRef :type Integer))
  (Utilities|Map|Add (.staticinteractablesdata (Utilities|Array|Get(acopy) (Variables|/Game/Game/SaveGame/BP_SaveGame.BP_SaveGame_C|GetLevelStates SaveGameRef) LevelDataRef)) (Utilities|String|StringToName (Utilities|GetObjectName self)) (Utilities|Struct|MakeST_InteractableData (Variables|Default|GetInteractable%20State) (Variables|Default|GetIsInteractable) (Variables|Default|Gettoll))))

(fn ConstructionScript
  (bind _text (Variables|Default|GetText))
  (bind _returnvalue (Utilities|GetDataTableRow "/Game/Game/Systems/Inventory/DT_Items.DT_Items" (Variables|Default|GetRow%20Name))
    (:then
      (Variables|Default|SetItemToCharge _returnvalue)
      (if (> (Variables|Default|Gettoll) 0)
        (Rendering|Components|TextRender|SetText _text (Utilities|Text|ToText(Integer) (Variables|Default|Gettoll)))
        (Components|StaticMesh|SetStaticMesh (Variables|Default|GetStaticMesh) (.mesh (Variables|Default|GetItemToCharge)))
        (else
          (Rendering|SetVisibility _text false false))))))

(fn CountasInteractable
  (return (Variables|Default|GetIsInteractable)))

(fn GetInteractLocation
  (return (Transformation|GetWorldLocation (Variables|Default|GetBox))))