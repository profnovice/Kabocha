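; Spline-following particle actor that relays an interaction to a target actor through a moving Niagara effect with sound.
; On Interact, a Timeline carries the effect along the spline, with play rate set from MoveSpeed divided by spline length to account for path length.
; When it finishes, it stops the audio, clears the effect and sends Interact to ActorToAffect.
; It reports itself as non-interactable, and its save and load events are empty.
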(event EventBeginPlay)

(event Collision|EventActorBeginOverlap
  (params (OtherActor :type Actor%20Object%20Reference)))

(event EventTick
  (params (DeltaSeconds :type Float%20%28single-precision%29)))

(event EventInteract
  (params (Interactor :type Actor%20Object%20Reference))
  (bind _spline (Variables|Default|GetSpline))
  (bind _audio (Variables|Default|GetAudio))
  (bind _returnvalue (Spline|GetSplineLength _spline))
  (Class|NiagaraComponent|SetAsset (Variables|Default|GetNiagara) "/Game/Game/Particle/NewNiagaraSystem1.NewNiagaraSystem1" true)
  (Components|Timeline|SetPlayRate (Variables|Default|GetTimeline) (/ (Variables|Default|GetMoveSpeed) _returnvalue))
  (Audio|Components|Audio|SetSound _audio "/Game/Game/Audio/SFX/welder-3-54547.welder-3-54547")
  (Audio|Components|Audio|Play _audio 0.0)
  (bind _newtrack_0 (Timeline|Timeline PlayFromStart)
    (:Update
      (Transformation|SetWorldLocation (Variables|Default|GetNiagara) (Spline|GetLocationatDistanceAlongSpline _spline (Math|Float|Lerp 0.0 _returnvalue _newtrack_0) "World") false false))
    (:Finished
      (Audio|Components|Audio|Stop (Variables|Default|GetAudio))
      (Class|NiagaraComponent|SetAsset (Variables|Default|GetNiagara) 0 true)
      (Class|BPIInteractable|Interact(Message) (Variables|Default|GetActorToAffect) self))))

(event EventLoadObjectData
  (params (SaveGameRef :type BP%20Save%20Game%20Object%20Reference) (LevelDataRef :type Integer)))

(event EventSaveObjectData
  (params (SaveGameRef :type BP%20Save%20Game%20Object%20Reference) (LevelDataRef :type Integer)))

(fn ConstructionScript)

(fn CountasInteractable
  (return false))

(fn GetInteractLocation
  (return (Transformation|GetWorldLocation (Variables|Default|GetCube))))