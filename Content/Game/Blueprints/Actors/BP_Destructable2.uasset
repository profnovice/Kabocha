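; BP_Destructable2 is a destructible dwarf actor that reacts to damage and death through its HealthComponent.
; Damage plays a clockwork-robot sound whose pitch rises with lost health plus random variation, while a timeline drives a morph-target reaction.
; Death shows the component's invisible message, plays a death sound and animates the same morph target before destroying the actor.
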(event OnDeath(HealthComponent)
  (Class|BPIHealthComponent|MakeInvisible(Message) (Variables|Default|GetHealthComponent))
  (Audio|PlaySoundatLocation "/Game/Game/Audio/SFX/DwarfDeath.DwarfDeath" (Transformation|GetActorLocation) "0, 0, 0" 0.2 1.0 0.0 0 0 0 0)
  (bind _dies (Timeline|Die PlayFromStart)
    (:Update
      (Components|SkeletalMesh|SetMorphTarget (Variables|Default|GetDwarf) "Key_1" _dies true))
    (:Finished
      (Actor|DestroyActor))))

(event OnDamageTaken(HealthComponent)
  (bind _healthcomponent (Variables|Default|GetHealthComponent))
  (bind _maxhealth (Variables|/Game/Game/Blueprints/Components/HealthComponent.HealthComponent_C|GetMaxHealth _healthcomponent))
  (if (not (Variables|/Game/Game/Blueprints/Components/HealthComponent.HealthComponent_C|GetIsDead (Variables|Default|GetHealthComponent)))
    (Audio|PlaySoundatLocation "/Game/Game/Audio/SFX/a_clockwork_robot___-_AudioTrimmer_com_.a_clockwork_robot___-_AudioTrimmer_com_" (Transformation|GetActorLocation) "0, 0, 0" 0.2 (+ (* (Math|Float|NormalizetoRange (- _maxhealth (Variables|/Game/Game/Blueprints/Components/HealthComponent.HealthComponent_C|GetHealth _healthcomponent)) 0.0 _maxhealth) 2.0) (Math|Random|RandomFloatinRange -0.1 0.4)) 0.0 0 0 0 0)
    (bind _react (Timeline|TakeDamage PlayFromStart)
      (:Update
        (Components|SkeletalMesh|SetMorphTarget (Variables|Default|GetDwarf) "Key_1" _react true)))))

(event EventBeginPlay)

(event Collision|EventActorBeginOverlap
  (params (OtherActor :type Actor%20Object%20Reference)))

(event EventTick
  (params (DeltaSeconds :type Float%20%28single-precision%29)))

(fn ConstructionScript)