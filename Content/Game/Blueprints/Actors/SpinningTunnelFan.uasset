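; Spinning tunnel fan actor that rotates its fan component and plays a large-fan sound.
; On BeginPlay it calls Spin and starts the sound on its Audio component, which plays regardless of ShouldSpin.
; Spin runs a timeline that drives the fan's relative pitch, then calls itself on finish, looping while ShouldSpin is true.
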(event Custom|Spin
  (if (Variables|Default|GetShouldSpin)
    (bind _newtrack_0 (Timeline|Timeline PlayFromStart)
      (:Update
        (Transformation|SetRelativeRotation (Variables|Default|GetTunnnelCircleFan) (Math|Rotator|MakeRotator 0.0 _newtrack_0 0.0) false false))
      (:Finished
        (CallFunction|Spin)))))

(event Custom|PlaySound
  (bind _audio (Variables|Default|GetAudio))
  (Audio|Components|Audio|SetSound _audio "/Game/Game/Audio/SFX/large-fan-38268.large-fan-38268")
  (Audio|Components|Audio|Play _audio 0.0))

(event EventBeginPlay
  (CallFunction|Spin)
  (CallFunction|PlaySound))

(event Collision|EventActorBeginOverlap
  (params (OtherActor :type Actor%20Object%20Reference)))

(event EventTick
  (params (DeltaSeconds :type Float%20%28single-precision%29)))

(fn ConstructionScript)