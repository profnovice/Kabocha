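; An interactable light post actor that players can switch on and off, with its state persisting through save games.
; Interacting flips the state enum, plays a switch sound and sets the intensity of two point lights.
; The construction script applies the StartAsOn default.
; On BeginPlay it requests a load from the game instance, then restores or saves its state in per-level save data keyed by object name.
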(event Custom|Update%20Physical%20State
  (bind _pointlight (Variables|Default|GetPointLight))
  (if (Utilities|Enum|Equal(Enum) (Variables|Default|GetInteractable%20State) "NewEnumerator4")
    (Rendering|Components|Light|SetIntensity _pointlight 5e+03)
    (else
      (Rendering|Components|Light|SetIntensity _pointlight 0.0))))

(event EventBeginPlay
  (Class|BPIPersistance|RequestLoad(Message) (Game|GetGameInstance) self))

(event EventLoadObjectData
  (params (SaveGameRef :type BP%20Save%20Game%20Object%20Reference) (LevelDataRef :type Integer))
  (bind _self self)
  (bind _levelstates (Variables|/Game/Game/SaveGame/BP_SaveGame.BP_SaveGame_C|GetLevelStates SaveGameRef))
  (bind _returnvalue (Utilities|GetObjectName _self))
  (bind _output (Utilities|Array|Get(acopy) _levelstates LevelDataRef))
  (bind _returnvalue_2 (Utilities|String|StringToName _returnvalue))
  (bind (_value _returnvalue_3) (Utilities|Map|Find (.staticinteractablesdata _output) _returnvalue_2))
  (if (.isvalid _output)
    (if _returnvalue_3
      (Variables|Default|SetInteractable%20State (.State (Utilities|Struct|BreakST_InteractableData _value)))
      (CallFunction|UpdatePhysicalState))))

(event EventSaveObjectData
  (params (SaveGameRef :type BP%20Save%20Game%20Object%20Reference) (LevelDataRef :type Integer))
  (Utilities|Map|Add (.staticinteractablesdata (Utilities|Array|Get(acopy) (Variables|/Game/Game/SaveGame/BP_SaveGame.BP_SaveGame_C|GetLevelStates SaveGameRef) LevelDataRef)) (Utilities|String|StringToName (Utilities|GetObjectName self)) (Utilities|Struct|MakeST_InteractableData (Variables|Default|GetInteractable%20State) true)))

(event EventInteract
  (params (Interactor :type Actor%20Object%20Reference))
  (if (Utilities|Enum|Equal(Enum) (Variables|Default|GetInteractable%20State) "NewEnumerator4")
    (Variables|Default|SetInteractable%20State "NewEnumerator5")
    (else
      (Variables|Default|SetInteractable%20State "NewEnumerator4")))
  (Audio|PlaySoundatLocation "/Game/Game/Audio/SFX/switch-150130.switch-150130" (Transformation|GetActorLocation) "0, 0, 0" 1.0 1.0 0.0 0 0 0 0)
  (CallFunction|UpdatePhysicalState))

(fn ConstructionScript
  (bind _pointlight (Variables|Default|GetPointLight))
  (if (Variables|Default|GetStartAsOn)
    (Variables|Default|SetInteractable%20State "NewEnumerator4")
    (else
      (Variables|Default|SetInteractable%20State "NewEnumerator5")))
  (if (Utilities|Enum|Equal(Enum) (Variables|Default|GetInteractable%20State) "NewEnumerator4")
    (Rendering|Components|Light|SetIntensity _pointlight 5e+03)
    (else
      (Rendering|Components|Light|SetIntensity _pointlight 0.0))))

(fn CountasInteractable
  (return true))

(fn GetInteractLocation
  (return (+ (Transformation|GetActorLocation) "0.000000,0.000000,100.000000")))