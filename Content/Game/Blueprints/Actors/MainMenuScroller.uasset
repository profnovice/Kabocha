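; MainMenuScroller is an actor that scrolls continuously along the X axis, apparently as moving scenery for the main menu.
; From BeginPlay, a self-restarting Timeline moves it with swept SetActorLocation calls, adding Speed times the track value to X on each update.
; When a Timeline pass finishes with X at or beyond EndDistance, it resets the actor's location before looping again.
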(event Custom|movementloop
  (bind _returnvalue (Transformation|GetActorTransform))
  (bind _newtrack_0 (Timeline|Timeline PlayFromStart)
    (:Update
      (Transformation|SetActorLocation (Math|Vector|MakeVector (+ (.x (.location _returnvalue)) (* (Variables|Default|GetSpeed) _newtrack_0)) (.y (.location _returnvalue)) (.z (.location _returnvalue))) true false))
    (:Finished
      (if (>= (.x (.location (Transformation|GetActorTransform))) (Variables|Default|GetEndDistance))
        (Transformation|SetActorLocation (Math|Vector|MakeVector 0.0 0.0 0.0) false false))
      (CallFunction|Movementloop))))

(event EventBeginPlay
  (CallFunction|Movementloop))

(event Collision|EventActorBeginOverlap
  (params (OtherActor :type Actor%20Object%20Reference)))

(event EventTick
  (params (DeltaSeconds :type Float%20%28single-precision%29)))

(fn ConstructionScript)