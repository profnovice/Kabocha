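; BP_SaveableDoor is an interactable door actor that keeps a two-value state across saves.
; Interaction toggles the state and calls UpdatePhysicalState, which so far only branches on it without moving anything.
; On BeginPlay it sends a load request to the GameInstance.
; Its save and load events store and restore the state in the save game's per-level static-interactables map, keyed by the actor's object name.
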(event Custom|UpdatePhysicalState
  (if (Utilities|Enum|Equal(Enum) (Variables|Default|GetInteractable%20State) "NewEnumerator0")
    _))

(event Custom|CustomEvent
  (params (Interactor :type Actor%20Object%20Reference))
  (if (Utilities|Enum|Equal(Enum) "NewEnumerator0" (Variables|Default|GetInteractable%20State))
    (Variables|Default|SetInteractable%20State "NewEnumerator1")
    (else
      (Variables|Default|SetInteractable%20State "NewEnumerator0")))
  (CallFunction|UpdatePhysicalState))

(event EventBeginPlay
  (Class|BPIPersistance|RequestLoad(Message) (Game|GetGameInstance) self))

(event Collision|EventActorBeginOverlap
  (params (OtherActor :type Actor%20Object%20Reference)))

(event EventTick
  (params (DeltaSeconds :type Float%20%28single-precision%29)))

(event EventLoadObjectData
  (params (SaveGameRef :type BP%20Save%20Game%20Object%20Reference) (LevelDataRef :type Integer))
  (bind _self self)
  (bind _levelstates (Variables|/Game/Game/SaveGame/BP_SaveGame.BP_SaveGame_C|GetLevelStates SaveGameRef))
  (bind _returnvalue (Utilities|GetObjectName _self))
  (bind _output (Utilities|Array|Get(acopy) _levelstates LevelDataRef))
  (bind _returnvalue_2 (Utilities|String|StringToName _returnvalue))
  (bind (_value _returnvalue_3) (Utilities|Map|Find (.staticinteractablesdata _output) _returnvalue_2))
  (if (.isvalid _output)
    (if _returnvalue_3
      (Variables|Default|SetInteractable%20State (Utilities|Struct|BreakST_InteractableData _value))
      (CallFunction|UpdatePhysicalState))))

(event EventSaveObjectData
  (params (SaveGameRef :type BP%20Save%20Game%20Object%20Reference) (LevelDataRef :type Integer))
  (Utilities|Map|Add (.staticinteractablesdata (Utilities|Array|Get(acopy) (Variables|/Game/Game/SaveGame/BP_SaveGame.BP_SaveGame_C|GetLevelStates SaveGameRef) LevelDataRef)) (Utilities|String|StringToName (Utilities|GetObjectName self)) (Utilities|Struct|MakeST_InteractableData (Variables|Default|GetInteractable%20State))))

(fn ConstructionScript)